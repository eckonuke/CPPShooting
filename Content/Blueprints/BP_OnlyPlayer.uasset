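; BP_OnlyPlayer is a player-controlled shooter that moves in the Y-Z plane and fires BP_OnlyBullet.
; Tick normalizes the Horizontal and Vertical input into a direction, then offsets the location by a fixed speed scaled by delta time, without sweep.
; Fire on release and FireTwo on press both spawn a bullet at the FirePos transform, the latter passing it as split location, rotation and scale.
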(event EventBeginPlay)

(event Collision|EventActorBeginOverlap
  (params (OtherActor :type Actor%20Object%20Reference)))

(event EventTick
  (params (DeltaSeconds :type Float%20%28single-precision%29))
  (Transformation|SetActorLocation (+ (* DeltaSeconds (* (Math|Vector|Normalize (Math|Vector|MakeVector 0.0 (Input|AxisValues|GetHorizontal) (Input|AxisValues|GetVertical))) (Math|Float|MakeLiteralFloat 5e+02))) (Transformation|GetActorLocation)) false false))

(event Input|ActionEvents|InputActionFire
  (params (Key :type Key%20Structure :default "None"))
  ;[1 1 1] 총알발사
  (:Released
    (Game|SpawnActorfromClass "/Game/Blueprints/BP_OnlyBullet.BP_OnlyBullet_C" (Transformation|GetWorldTransform (Variables|Default|GetFirePos)) "Undefined" 0 0)))

(event Input|ActionEvents|InputActionFireTwo
  (params (Key :type Key%20Structure :default "None"))
  (bind _firepos (Variables|Default|GetFirePos))
  (bind _returnvalue (Transformation|GetWorldTransform _firepos))
  ;[1 1 1] 총알발사
  (:Pressed
    (Game|SpawnActorfromClass "/Game/Blueprints/BP_OnlyBullet.BP_OnlyBullet_C" (Math|Transform|MakeTransform (.location _returnvalue) (.rotation _returnvalue) (.scale _returnvalue)) "Undefined" 0 0)))

(fn ConstructionScript)